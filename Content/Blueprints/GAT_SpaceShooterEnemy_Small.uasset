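; Small enemy for a space shooter that flips 180 degrees on spawn and moves along its local Y axis at Speed, with sweep.
; Box1 overlaps map three ammo classes to A, B and C marker begin/end calls, storing the ammo on begin.
; DestroyOverlappedActor spawns an explosion at that stored ammo and destroys it, leaving the enemy intact.
; Health, score, ammo and weapon getters are stubs returning zero.
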(event OnComponentEndOverlap(Box1)
  (params (OtherActor :type Actor%20Object%20Reference) (OtherComp :type Primitive%20Component%20Object%20Reference) (OtherBodyIndex :type Integer))
  (bind _returnvalue (Utilities|GetClass OtherActor))
  (if (== _returnvalue "/Game/Blueprints/GAT_SpaceShooterAmmo02.GAT_SpaceShooterAmmo02_C")
    (Default|CallEndAMarkerOverlap)
    (elif (== _returnvalue "/Game/Blueprints/GAT_SpaceShooterAmmo01.GAT_SpaceShooterAmmo01_C")
      (Default|CallEndBMarkerOverlap)
      (elif (== _returnvalue "/Game/Blueprints/GAT_SpaceShooterAmmo03.GAT_SpaceShooterAmmo03_C")
        (Default|CallEndCMarkerOverlap)))))

(event OnComponentBeginOverlap(Box1)
  (params (OtherActor :type Actor%20Object%20Reference) (OtherComp :type Primitive%20Component%20Object%20Reference) (OtherBodyIndex :type Integer) (bFromSweep :type Boolean) (SweepResult :type Hit%20Result%20Structure%20%28by%20ref%29))
  (bind _returnvalue (Utilities|GetClass OtherActor))
  (if (== _returnvalue "/Game/Blueprints/GAT_SpaceShooterAmmo02.GAT_SpaceShooterAmmo02_C")
    (Default|CallAMarkerOverlap)
    (Variables|Default|SetOverlappedActor OtherActor :!label _label)
    (elif (== _returnvalue "/Game/Blueprints/GAT_SpaceShooterAmmo01.GAT_SpaceShooterAmmo01_C")
      (Default|CallBMarkerOverlap)
      (goto _label)
      (elif (== _returnvalue "/Game/Blueprints/GAT_SpaceShooterAmmo03.GAT_SpaceShooterAmmo03_C")
        (Default|CallCMarkerOverlap)
        (goto _label)))))

(event Custom|DestroyOverlappedActor
  (bind _overlappedactor (Variables|Default|GetOverlappedActor))
  (Effects|SpawnEmitteratLocation "/Game/Particles/P_Explosion.P_Explosion" (Transformation|GetActorLocation _overlappedactor))
  (Actor|DestroyActor _overlappedactor))

(event EventTick
  (params (DeltaSeconds :type Float%20%28single-precision%29))
  (Transformation|AddActorLocalOffset (Math|Vector|MakeVector 0.0 (* DeltaSeconds (Variables|Default|GetSpeed)) 0.0) true))

(event EventBeginPlay
  (Transformation|SetActorRotation "0.000000,180.000000, 0"))

(fn ConstructionScript)

(fn GetPlayerHealth
  (return 0))

(fn GetScore
  (return 0))

(fn GetAmmoCount
  (return 0))

(fn GetWeaponTYpe
  (return 0))