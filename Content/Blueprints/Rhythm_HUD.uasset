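; HUD for a rhythm game that draws all its text on the canvas in DrawHUD, with a layout chosen by GameMode.
; Mode 0 shows score, A/S/D key labels and a central call-and-response prompt (Listen, YourTurn or Game Over) driven by display flags; mode 1 shows only score.
; EnemyDestroyedUpdateScore adds to the score and clamps it at zero.
; The health, score, ammo and weapon getters are stubs returning zero.
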(event EventEnemyDestroyedUpdateScore
  (params (ScoreValue :type Integer))
  (Variables|Default|SetScore (+ ScoreValue (Variables|Default|GetScore)))
  (if (< (Variables|Default|GetScore) 0)
    (Variables|Default|SetScore 0)))

(event EventDrawHUD
  (params (SizeX :type Integer) (SizeY :type Integer))
  (bind _listen (Variables|Default|GetListen))
  (bind _yourturn (Variables|Default|GetYourTurn))
  (Variables|Default|SetScreenDimensions (Math|Vector2D|MakeVector2D (Math|Conversions|ToFloat(Integer) SizeX) (Math|Conversions|ToFloat(Integer) SizeY)))
  (switch int (Variables|Default|GetGameMode)
    (:0
      (HUD|DrawText (Utilities|String|ToString(Integer) (Variables|Default|GetScore)) "(R=0.023159,G=1.000000,B=0.000000,A=1.000000)" (* (.X (Math|Vector2D|BreakVector2D (Variables|Default|GetScreenDimensions))) 0.1) 2e+01 "/Engine/EngineFonts/RobotoDistanceField.RobotoDistanceField" 2.0 false)
      (HUD|DrawText "= A" "(R=0.023159,G=1.000000,B=0.000000,A=1.000000)" (* (.X (Math|Vector2D|BreakVector2D (Variables|Default|GetScreenDimensions))) 0.25) (* (.Y (Math|Vector2D|BreakVector2D (Variables|Default|GetScreenDimensions))) 0.8) "/Engine/EngineFonts/RobotoDistanceField.RobotoDistanceField" 2.0 false)
      (HUD|DrawText "= S" "(R=0.023159,G=1.000000,B=0.000000,A=1.000000)" (* (.X (Math|Vector2D|BreakVector2D (Variables|Default|GetScreenDimensions))) 0.54) (* (.Y (Math|Vector2D|BreakVector2D (Variables|Default|GetScreenDimensions))) 0.8) "/Engine/EngineFonts/RobotoDistanceField.RobotoDistanceField" 2.0 false)
      (HUD|DrawText "= D" "(R=0.023159,G=1.000000,B=0.000000,A=1.000000)" (* (.X (Math|Vector2D|BreakVector2D (Variables|Default|GetScreenDimensions))) 0.825) (* (.Y (Math|Vector2D|BreakVector2D (Variables|Default|GetScreenDimensions))) 0.8) "/Engine/EngineFonts/RobotoDistanceField.RobotoDistanceField" 2.0 false)
      (if (Variables|Default|GetDisplayGameOver)
        (HUD|DrawText "Game Over" "(R=0.023159,G=1.000000,B=0.000000,A=1.000000)" (- (* (.X (Math|Vector2D|BreakVector2D (Variables|Default|GetScreenDimensions))) 0.5) (/ (.OutWidth (Class|HUD|GetTextSize _listen "/Engine/EngineFonts/RobotoDistanceField.RobotoDistanceField" 2.0)) 2.0)) (* (.Y (Math|Vector2D|BreakVector2D (Variables|Default|GetScreenDimensions))) 0.5) "/Engine/EngineFonts/RobotoDistanceField.RobotoDistanceField" 3.0 false)
        (elif (Variables|Default|GetDisplayCall)
          (HUD|DrawText _listen "(R=0.023159,G=1.000000,B=0.000000,A=1.000000)" (- (* (.X (Math|Vector2D|BreakVector2D (Variables|Default|GetScreenDimensions))) 0.5) (/ (.OutWidth (Class|HUD|GetTextSize _listen "/Engine/EngineFonts/RobotoDistanceField.RobotoDistanceField" 2.0)) 2.0)) (* (.Y (Math|Vector2D|BreakVector2D (Variables|Default|GetScreenDimensions))) 0.5) "/Engine/EngineFonts/RobotoDistanceField.RobotoDistanceField" 3.0 false)
          (else
            (HUD|DrawText _yourturn "(R=0.023159,G=1.000000,B=0.000000,A=1.000000)" (- (* (.X (Math|Vector2D|BreakVector2D (Variables|Default|GetScreenDimensions))) 0.5) (/ (.OutWidth (Class|HUD|GetTextSize _yourturn "/Engine/EngineFonts/RobotoDistanceField.RobotoDistanceField" 2.0)) 2.0)) (* (.Y (Math|Vector2D|BreakVector2D (Variables|Default|GetScreenDimensions))) 0.5) "/Engine/EngineFonts/RobotoDistanceField.RobotoDistanceField" 3.0 false)))))
    (:1
      (HUD|DrawText (Utilities|String|ToString(Integer) (Variables|Default|GetScore)) "(R=0.023159,G=1.000000,B=0.000000,A=1.000000)" (* (.X (Math|Vector2D|BreakVector2D (Variables|Default|GetScreenDimensions))) 0.15) 2e+01 "/Engine/EngineFonts/RobotoDistanceField.RobotoDistanceField" 2.0 false))))

(fn ConstructionScript)

(fn GetPlayerHealth
  (return 0))

(fn GetScore
  (return 0))

(fn GetAmmoCount
  (return 0))

(fn GetWeaponTYpe
  (return 0))